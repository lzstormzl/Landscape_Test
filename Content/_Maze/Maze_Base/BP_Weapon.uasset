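; BP_Weapon is a weapon actor with a spear that deals point damage to the actors it hits.
; On BeginPlay it passes the Spear to its collision component and adds its owner to that component's ignore list.
; When the component fires DamageActor, the weapon applies fixed point damage along the owner's forward vector, crediting the instigator's controller.
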(event `self.ReceiveBeginPlay`
  (`/Game/_Maze/Maze_Base/Components/AC_WeaponCollision.Set Weapon` (`self.AC_Collision`) (`self.Spear`))
  (`KismetArrayLibrary.Array_Add` (`/Game/_Maze/Maze_Base/Components/AC_WeaponCollision.Actors to Ignore` (`self.AC_Collision`)) (`self.GetOwner`)))

(event `self.AC_Collision.Damage Actor`
  (params (HitData :type "HitResult Structure"))
  (`GameplayStatics.ApplyPointDamage` (`.HitActor` (`GameplayStatics.BreakHitResult` HitData)) 20.0 (`self.GetActorForwardVector` (`self.GetOwner`)) HitData (`self.GetInstigatorController`) self))

(fn `UserConstructionScript`)