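; Weapon collision component that detects hits along a weapon during attacks and reports each struck actor.
; While collision is on, Tick runs a multi-sphere object trace between the start and end sockets of the assigned weapon.
; An already-hit list, cleared whenever collision turns on, limits each actor to one CallDamageActor dispatch per activation window.
; External callers set the weapon and toggle collision on and off.
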(event `CollisionTrace`
  (bind _weapon (`self.Weapon`))
  (bind _outhits (`KismetSystemLibrary.SphereTraceMultiForObjects` (`SceneComponent.GetSocketLocation` _weapon (`self.StartSocket`)) (`SceneComponent.GetSocketLocation` _weapon (`self.EndSocket`)) (`self.Radius`) (`self.Object Types`) false (`self.Actors to Ignore`) (`self.Draw Debug Type`)))
  (for _array_element _outhits
    (bind _output_get (set `self.LastHit` _array_element))
    (bind (_bblockinghit _binitialoverlap _time _distance _location _impactpoint _normal _impactnormal _physmat _hitactor) (`GameplayStatics.BreakHitResult` _output_get))
    (bind _returnvalue (`self.Can Hit Actor` _hitactor))
    (if _returnvalue
      (bind _output_get_2 (set `self.Hit Actor` _hitactor))
      (`KismetArrayLibrary.Array_Add` (`self.AlreadyHit?`) _output_get_2)
      (`self.Damage Actor` (`self.LastHit`)))))

(event `self.ReceiveTick`
  (params (DeltaSeconds :type "Float (single-precision)"))
  (if (`self.CollisionOn?`)
    (`self.CollisionTrace`)))

(event `TurnOnCollision`
  (`self.ClearHitActor`)
  (set `self.CollisionOn?` true))

(event `ClearHitActor`
  (`KismetArrayLibrary.Array_Clear` (`self.AlreadyHit?`)))

(event `TurnOffCollision`
  (set `self.CollisionOn?` false))

(event `Set Weapon`
  (params (Weapon :type "PrimitiveComponent Object Reference"))
  (set `self.Weapon` Weapon))

(fn `Can Hit Actor`
  (params (Actor :type "Actor Object Reference"))
  (returns (ReturnValue :type Boolean))
  (return (not (`KismetArrayLibrary.Array_Contains` (`self.AlreadyHit?`) Actor))))