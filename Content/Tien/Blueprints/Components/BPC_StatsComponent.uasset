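; Stats component that tracks health, stamina and focus for its owner and drives the player HUD or boss health bar by actor tag.
; Consume and add functions update values and bars, and full focus converts into focus points.
; Looping named timers regenerate stamina and lerp the secondary health and stamina bars after a short delay.
; ConsumeFocusPoint clamps to a zero range, so any spend empties all points.
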(event `self.ReceiveBeginPlay`)

(event `HealthBar2LerpEvent`
  ;[0 0.01562 1] Health bar 2 lerp event
  (`KismetSystemLibrary.K2_PauseTimer` null "HealthBar2Lerp")
  (`KismetSystemLibrary.Delay` 1.5)
  (`KismetSystemLibrary.K2_SetTimer` null "HealthBar2Lerp" 0.1 true))

(event `RegenStaminaEvent`
  ;[1 0.3281 0 0.5] Regen Stamina Event
  (`KismetSystemLibrary.K2_PauseTimer` null "StaminaRegen")
  (bind _playerstate (message `/Game/Tien/Blueprints/Interface/BPI_Stats.GetPlayerCurrentState` (`self.GetOwner`)))
  (if (`|EnumEquality` _playerstate "NewEnumerator0")
    (`KismetSystemLibrary.K2_SetTimer` null "StaminaRegen" 0.5 true)
    (else
      (`KismetSystemLibrary.PrintString` "?????"))))

(event `StaminaBar2LerpEvent`
  ;[1 0 0] Lerp Stamina Bar 2
  (`KismetSystemLibrary.K2_PauseTimer` null "StaminaBar2Lerp")
  (`KismetSystemLibrary.Delay` 0.1)
  (`KismetSystemLibrary.K2_SetTimer` null "StaminaBar2Lerp" 0.01 true))

(fn `BossHealthBarUpdate`
  (bind _bosshealthbar (`self.BossHealthBar`))
  (`/Engine/EditorBlueprintResources/StandardMacros.IsValid` _bosshealthbar
    (:`Is Valid`
      (`ProgressBar.SetPercent` _bosshealthbar (`self.HealthPercent`)))
    (:`Is Not Valid`
      (`KismetSystemLibrary.PrintString` "Chưa có boss health bar"))))

(fn `ConsumeFocusPoint`
  (params (Consume :type Integer))
  (returns (ConsumValue :type Integer))
  (locals (LastCurrentFocusPoint :type Integer))
  (bind _currentfocuspoint (`self.CurrentFocusPoint`))
  (set `local.LastCurrentFocusPoint` (`self.CurrentFocusPoint`))
  (`|ExecutionSequence`
    (:`then_0`
      (if (> Consume (`self.CurrentFocusPoint`))
        (set `self.CurrentFocusPoint` (`KismetMathLibrary.Clamp` (- Consume (`self.CurrentFocusPoint`))))
        (`self.UpdateFocusPointUI`)
        (return (`local.LastCurrentFocusPoint`))))
    (:`then_1`
      (if (== Consume _currentfocuspoint)
        (set `self.CurrentFocusPoint` (`KismetMathLibrary.Clamp` (- Consume _currentfocuspoint)))
        (`self.UpdateFocusPointUI`)
        (return Consume)))
    (:`then_2`
      (set `self.CurrentFocusPoint` (`KismetMathLibrary.Clamp` (- (`self.CurrentFocusPoint`) Consume)))
      (`self.UpdateFocusPointUI`)
      (return Consume))))

(fn `ConsumeStamina`
  (params (StaminaCost :type "Float (double-precision)"))
  (returns (`New Value Stamina` :type "Float (double-precision)"))
  (bind _returnvalue (/ (`self.CurrentStamina`) (`self.MaxStamina`)))
  (message `/Game/Tien/Blueprints/Interface/BPI_Player.StopBlueStaminaTimeLine` (`self.GetOwner`))
  (bind _output_get (set `self.CurrentStamina` (`KismetMathLibrary.FClamp` (- (`self.CurrentStamina`) StaminaCost) 0.0 (`self.MaxStamina`))))
  (`self.StaminaBarUpdate` _returnvalue)
  (`self.StaminaBar3Update` _returnvalue)
  (return _output_get))

(fn `CreateBossStatBar`
  (bind _returnvalue (`|CreateWidget` "/Game/Tien/Widgets/WD_Boss_Health.WD_Boss_Health_C" (`GameplayStatics.GetPlayerController` 0)))
  (bind _output_get (set `self.BossStatBar` _returnvalue))
  (`UserWidget.AddToViewport` _output_get 0)
  (`self.SetBossStatBar`))

(fn `FocusBarUpdate`
  (bind _focusbar (`self.FocusBar`))
  (`/Engine/EditorBlueprintResources/StandardMacros.IsValid` _focusbar
    (:`Is Valid`
      (`ProgressBar.SetPercent` _focusbar (/ (`self.CurrentFocus`) (`self.MaxFocus`)))
      (return))))

(fn `HealthBar2Lerp`
  (bind _healthbar2 (`self.HealthBar2`))
  (bind _returnvalue (/ (`self.CurrentHealth`) (`self.MaxHealth`)))
  (bind _percent (`ProgressBar.Percent` _healthbar2))
  (`/Engine/EditorBlueprintResources/StandardMacros.IsValid` _healthbar2
    (:`Is Valid`
      (if (`KismetMathLibrary.NearlyEqual_FloatFloat` _percent _returnvalue 0.001)
        (`KismetSystemLibrary.K2_PauseTimer` null "HealthBar2Lerp")
        (return)
        (else
          (`ProgressBar.SetPercent` (`self.HealthBar2`) (`KismetMathLibrary.Lerp` _percent _returnvalue 0.2))
          (return))))
    (:`Is Not Valid`
      (`KismetSystemLibrary.K2_PauseTimer` null "HealthBar2Lerp")
      (return))))

(fn `HealthBar2Update`
  (bind _healthbar2 (`self.HealthBar2`))
  (`/Engine/EditorBlueprintResources/StandardMacros.IsValid` _healthbar2
    (:`Is Valid`
      (`ProgressBar.SetPercent` _healthbar2 (/ (`self.CurrentHealth`) (`self.MaxHealth`)))
      (return))))

(fn `HealthBarUpdate`
  (bind _returnvalue (`self.GetOwner`))
  (bind _healthbar (`self.HealthBar`))
  (if (`Actor.ActorHasTag` _returnvalue "Player")
    (`/Engine/EditorBlueprintResources/StandardMacros.IsValid` _healthbar
      (:`Is Valid`
        (`ProgressBar.SetPercent` _healthbar (/ (`self.CurrentHealth`) (`self.MaxHealth`)))
        (return)))
    (elif (`Actor.ActorHasTag` _returnvalue "Boss")
      (`self.BossHealthBarUpdate`)
      (`KismetSystemLibrary.PrintString` "Update Boss health Bar"))))

(fn `InitializeStatsComponent`
  (bind _returnvalue (`self.StaminaPercent`))
  ;[1 1 1] Tạo widget dựa trên Tag
  (if (`Actor.ActorHasTag` (`self.GetOwner`) "Player")
    ;[0.1795 0.6056 1] Tạo HUD cho Player
    (bind _returnvalue_2 (`|CreateWidget` "/Game/Tien/Widgets/UserInterfaces/Widgets/MainHUD.MainHUD_C" (`GameplayStatics.GetPlayerController` 0)))
    (bind _output_get (set `self.MainHUDWidget` _returnvalue_2))
    (`UserWidget.AddToViewport` _output_get 0)
    ;[1 1 1] Tạo biến stats trong widget
    (`self.SetPlayerStatBar`)
    ;[1 1 1] Update Health Bar
    (`self.HealthBarUpdate`)
    (`self.HealthBar2Update`)
    ;[1 1 1] Update Stamina Bar
    (`self.StaminaBarUpdate` _returnvalue)
    (`self.StaminaBar2Update` _returnvalue)
    (`self.StaminaBar3Update` _returnvalue)
    ;[1 1 1] Update Focus Bar
    (`self.FocusBarUpdate`)))

(fn `InscreaseFocusPoint`
  (params (Value :type Integer))
  (bind _output_get (set `self.CurrentFocusPoint` (`KismetMathLibrary.Clamp` (+ Value (`self.CurrentFocusPoint`)) 0 (`self.MaxFocusPoint`))))
  (`self.UpdateFocusPointUI`)
  (`KismetSystemLibrary.PrintString` (`KismetStringLibrary.Concat_StrStr` "Focus Point: " (`KismetStringLibrary.Conv_IntToString` _output_get)))
  (if (== (`self.CurrentFocusPoint`) (`self.MaxFocusPoint`))
    (`self.FocusBarUpdate`)
    (return)
    (else
      (return))))

(fn `PlusFocus`
  (params (Amount :type "Float (double-precision)"))
  (returns (`New Value Stamina` :type "Float (double-precision)"))
  (if (== (`self.CurrentFocusPoint`) (`self.MaxFocusPoint`))
    (return 0.0)
    (else
      (bind _output_get (set `self.CurrentFocus` (+ (`self.CurrentFocus`) Amount)))
      (if (>= (`self.CurrentFocus`) (`self.MaxFocus`))
        (set `self.CurrentFocus` (- (`self.CurrentFocus`) (`self.MaxFocus`)))
        (`self.InscreaseFocusPoint` 1)
        (`self.FocusBarUpdate`)
        (else
          (`self.FocusBarUpdate`)
          (`KismetSystemLibrary.PrintString` (`KismetStringLibrary.Concat_StrStr` "Focus: " (`KismetStringLibrary.Conv_DoubleToString` _output_get)) true false (struct :`G` 0.66 :`B` 1.0 :`A` 1.0) 0.0)))
      (return (`self.CurrentFocus`)))))

(fn `PlusStamina`
  (params (Amount :type "Float (double-precision)"))
  (returns (`New Value Stamina` :type "Float (double-precision)"))
  (bind _output_get (set `self.CurrentStamina` (`KismetMathLibrary.FClamp` (+ (`self.CurrentStamina`) Amount) 0.0 (`self.MaxStamina`))))
  (`self.StaminaBarUpdate` (/ (`self.CurrentStamina`) (`self.MaxStamina`)))
  (return _output_get))

(fn `SetBossStatBar`
  (bind _bossstatbar (`self.BossStatBar`))
  (`/Engine/EditorBlueprintResources/StandardMacros.IsValid` _bossstatbar
    (:`Is Valid`
      (set `self.BossHealthBar` (`/Game/Tien/Widgets/WD_Boss_Health.BossHealth` _bossstatbar))
      (set `self.BossName` (`/Game/Tien/Widgets/WD_Boss_Health.BossName` _bossstatbar)))))

(fn `SetCurrentStaminaByPercent`
  (params (Percent :type "Float (double-precision)"))
  (set `self.CurrentStamina` (* Percent (`self.MaxStamina`))))

(fn `SetPlayerStatBar`
  (bind _mainhudwidget (`self.MainHUDWidget`))
  (`/Engine/EditorBlueprintResources/StandardMacros.IsValid` _mainhudwidget
    (:`Is Valid`
      (set `self.HealthBar` (`/Game/Tien/Widgets/UserInterfaces/Widgets/MainHUD.Health` _mainhudwidget))
      (set `self.HealthBar2` (`/Game/Tien/Widgets/UserInterfaces/Widgets/MainHUD.Health2` _mainhudwidget))
      (set `self.StaminaBar` (`/Game/Tien/Widgets/UserInterfaces/Widgets/MainHUD.Stamina` _mainhudwidget))
      (set `self.StaminaBar2` (`/Game/Tien/Widgets/UserInterfaces/Widgets/MainHUD.Stamina2` _mainhudwidget))
      (set `self.StaminaBar3` (`/Game/Tien/Widgets/UserInterfaces/Widgets/MainHUD.Stamina3` _mainhudwidget))
      (set `self.FocusBar` (`/Game/Tien/Widgets/UserInterfaces/Widgets/MainHUD.Focus` _mainhudwidget))
      (set `self.FocusPointPanel` (`/Game/Tien/Widgets/UserInterfaces/Widgets/MainHUD.FocusPointPanel` _mainhudwidget)))))

(fn `StaminaBar2Lerp`
  (bind _staminabar2 (`self.StaminaBar2`))
  (bind _returnvalue (/ (`self.CurrentStamina`) (`self.MaxStamina`)))
  (bind _percent (`ProgressBar.Percent` _staminabar2))
  (`/Engine/EditorBlueprintResources/StandardMacros.IsValid` _staminabar2
    (:`Is Valid`
      (if (`KismetMathLibrary.NearlyEqual_FloatFloat` _percent _returnvalue 0.001)
        (`KismetSystemLibrary.K2_PauseTimer` null "StaminaBar2Lerp")
        (else
          (`ProgressBar.SetPercent` _staminabar2 (`KismetMathLibrary.Lerp` _percent _returnvalue 0.2))
          (return))))))

(fn `StaminaBar2Update`
  (params (InPercent :type "Float (single-precision)"))
  (bind _staminabar2 (`self.StaminaBar2`))
  (`/Engine/EditorBlueprintResources/StandardMacros.IsValid` _staminabar2
    (:`Is Valid`
      (`ProgressBar.SetPercent` _staminabar2 InPercent)
      (return))))

(fn `StaminaBar3Update`
  (params (Percent :type "Float (double-precision)"))
  (bind _staminabar3 (`self.StaminaBar3`))
  (`/Engine/EditorBlueprintResources/StandardMacros.IsValid` _staminabar3
    (:`Is Valid`
      (`ProgressBar.SetPercent` _staminabar3 Percent)
      (return))))

(fn `StaminaBarUpdate`
  (params (InPercent :type "Float (single-precision)"))
  (bind _staminabar (`self.StaminaBar`))
  (`/Engine/EditorBlueprintResources/StandardMacros.IsValid` _staminabar
    (:`Is Valid`
      (`ProgressBar.SetPercent` _staminabar InPercent)
      (return))))

(fn `StaminaRegen`
  (bind _staminabar2 (`self.StaminaBar2`))
  (if (`self.bCanRegenStamina?`)
    (if (>= (`self.CurrentStamina`) (`self.MaxStamina`))
      (`KismetSystemLibrary.K2_PauseTimer` null "StaminaRegen")
      (set `self.CurrentStamina` (`self.MaxStamina`))
      (`self.StaminaBar2Update` (`self.StaminaPercent`))
      (else
        (set `self.CurrentStamina` (+ (`self.CurrentStamina`) (`self.StaminaRegenRate`)))
        (`self.StaminaBarUpdate` (`self.StaminaPercent`))
        (`self.StaminaBar3Update` (`self.StaminaPercent`))
        (`/Engine/EditorBlueprintResources/StandardMacros.IsValid` _staminabar2
          (:`Is Valid`
            (if (< (`ProgressBar.Percent` _staminabar2) (`self.StaminaPercent`))
              (`self.StaminaBar2Update` (`self.StaminaPercent`))
              (return))))))
    (else
      (`KismetSystemLibrary.K2_PauseTimer` null "StaminaRegen")
      (`KismetSystemLibrary.PrintString` "Hello"))))

(fn `Update Stamina 32By1Percent`
  (bind _percent (`ProgressBar.Percent` (`self.StaminaBar`)))
  (`self.StaminaBar2Update` _percent)
  (`self.StaminaBar3Update` _percent)
  (return))

(fn `UpdateFocusPointUI`
  (bind _focuspointpanel (`self.FocusPointPanel`))
  (`/Engine/EditorBlueprintResources/StandardMacros.IsValid` _focuspointpanel
    (:`Is Valid`
      (set `EditableTextBox.Text` (`KismetTextLibrary.Conv_IntToText` (`self.CurrentFocusPoint`)) _focuspointpanel))
    (:`Is Not Valid`
      (`KismetSystemLibrary.PrintString` "Không tìm thấy Focus Point Panel")))
  (return))