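; BPC_DamageSystem is an actor component that resolves incoming damage against the owner's BPC_StatsComponent health.
; TakeDamage uses the CanBeDamaged macro to route each hit to block, damage or no damage, based on dead, invincible and blocking states plus per-hit flags.
; It fires blocked, death or damage-response callbacks and returns whether damage landed.
; Non-lethal hits update health bars and trigger responses only when interruptible or force-interrupting.
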(event `self.ReceiveBeginPlay`
  (set `self.BPC_StatsComponents` (`Actor.GetComponentByClass` (`self.GetOwner`) "/Game/Tien/Blueprints/Components/BPC_StatsComponent.BPC_StatsComponent_C")))

(fn `TakeDamage`
  (params (DamageInfo :type "/Game/Tien/Blueprints/Struct/S_DamageInfo Structure"))
  (returns (IsDamaged :type Boolean))
  (bind (_amount _damagetype _damageresponse _shoulddamageinvincible _canbeblock _canbeparried _shouldforceinterrupt) (break `/Game/Tien/Blueprints/Struct/S_DamageInfo` DamageInfo))
  (bind _bpc_statscomponents (`self.BPC_StatsComponents`))
  (`self.CanBeDamaged` _shoulddamageinvincible _canbeblock
    (:`Block Damage`
      (`self.OnBlocked` _canbeparried)
      (return false))
    (:`Do Damage`
      (bind _output_get (set `/Game/Tien/Blueprints/Components/BPC_StatsComponent.CurrentHealth` (- (`/Game/Tien/Blueprints/Components/BPC_StatsComponent.CurrentHealth` (`self.BPC_StatsComponents`)) _amount) (`self.BPC_StatsComponents`)))
      (if (<= _output_get 0.0)
        (set `self.IsDead` true)
        (`/Game/Tien/Blueprints/Components/BPC_StatsComponent.HealthBarUpdate` _bpc_statscomponents)
        (`/Game/Tien/Blueprints/Components/BPC_StatsComponent.HealthBar2LerpEvent` _bpc_statscomponents)
        (`self.OnDeath`)
        (return true)
        (elif (or (`self.IsInterruptible`) _shouldforceinterrupt)
          (`/Game/Tien/Blueprints/Components/BPC_StatsComponent.HealthBarUpdate` _bpc_statscomponents)
          (`/Game/Tien/Blueprints/Components/BPC_StatsComponent.HealthBar2LerpEvent` _bpc_statscomponents)
          (`self.OnDamagedResponse` _damageresponse)
          (return true)
          (else
            (return true)))))
    (:`No Damage`
      (return false))))