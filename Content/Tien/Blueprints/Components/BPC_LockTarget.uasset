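; Lock-on targeting component for the BP_ThuyTinhTien player character.
; LockTarget toggles: it sphere-traces pawns along the camera's forward vector, then switches the character to controller-facing rotation and attaches a BP_TargetLock marker to the hit actor's root.
; Toggling off restores movement-oriented rotation and destroys the marker, though IsInCombat is set true either way.
; While locked, Tick snaps control rotation toward the target.
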(event `self.ReceiveBeginPlay`
  (bind _asbp_thuy_tinh_tien (cast `/Game/Tien/Characters/Player/BP_ThuyTinhTien` (`self.GetOwner`)))
  (set `self.PlayerThuyTinhTien` _asbp_thuy_tinh_tien))

(event `LockTarget`
  (bind _transformcomponent (`PlayerCameraManager.TransformComponent` (`GameplayStatics.GetPlayerCameraManager` 0)))
  (bind _charactermovement (`Character.CharacterMovement` (`GameplayStatics.GetPlayerCharacter` 0)))
  (bind _returnvalue (`SceneComponent.K2_GetComponentLocation` _transformcomponent))
  (`self.TargetLockActor`
    (:`then`
      (set `self.IsInCombat` true)
      (set `self.TargetLockActor` null)
      (set `CharacterMovementComponent.bOrientRotationToMovement` true _charactermovement)
      (set `CharacterMovementComponent.bUseControllerDesiredRotation` false _charactermovement)
      (`Actor.K2_DestroyActor` (`self.TargetLockIcon`)))
    (:`else`
      (bind (_outhit _returnvalue_2) (`KismetSystemLibrary.SphereTraceSingleForObjects` _returnvalue (+ _returnvalue (* (`KismetMathLibrary.GetForwardVector` (`SceneComponent.K2_GetComponentRotation` _transformcomponent)) 1000.0)) 150.0 (`|MakeArray` "ObjectTypeQuery3" :!type "EObjectTypeQuery Enum")))
      (if _returnvalue_2
        (set `self.IsInCombat` true)
        (set `self.TargetLockActor` (`.HitActor` (`GameplayStatics.BreakHitResult` _outhit)))
        (set `CharacterMovementComponent.bOrientRotationToMovement` false _charactermovement)
        (set `CharacterMovementComponent.bUseControllerDesiredRotation` true _charactermovement)
        (bind _returnvalue_3 (`|SpawnActorFromClass` "/Game/Tien/Blueprints/BP_TargetLock.BP_TargetLock_C" (`KismetMathLibrary.MakeTransform` (0.0 0.0 0.0)) "AlwaysSpawn" "MultiplyWithRoot" null null))
        (bind _output_get (set `self.TargetLockIcon` _returnvalue_3))
        (`Actor.K2_AttachToComponent` _output_get (`Actor.RootComponent` (`self.TargetLockActor`)) "Pelvis" "SnapToTarget" "SnapToTarget" "SnapToTarget" true)))))

(event `self.ReceiveTick`
  (params (DeltaSeconds :type "Float (single-precision)"))
  (`self.TargetLockActor`
    (:`then`
      (`Controller.SetControlRotation` (`Pawn.GetController` (`self.PlayerThuyTinhTien`)) (`KismetMathLibrary.FindLookAtRotation` (`Actor.K2_GetActorLocation` (`self.PlayerThuyTinhTien`)) (`Actor.K2_GetActorLocation` (`self.TargetLockActor`)))))
    (:`else`)))