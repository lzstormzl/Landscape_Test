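; Anim notify state that makes an enemy focus on its target during a window of an animation.
; On begin, it casts the mesh owner to BP_Enemy_Base and passes the ActorTarget from that enemy's AI controller to the owner through a Set Focus message.
; On end, it sends a Clear Focus message to the owner without casting.
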(fn `Received_NotifyBegin`
  (params (MeshComp :type "SkeletalMeshComponent Object Reference") (Animation :type "AnimSequenceBase Object Reference") (TotalDuration :type "Float (single-precision)") (EventReference :type "AnimNotifyEventReference Structure (by ref)"))
  (returns (ReturnValue :type Boolean))
  (bind _returnvalue (`ActorComponent.GetOwner` MeshComp))
  (`/Engine/EditorBlueprintResources/StandardMacros.IsValid` _returnvalue
    (:`Is Valid`
      (bind _asbp_enemy_base (cast `/Game/Tien/Characters/Enemy/BP_Enemy_Base` _returnvalue))
      (message `/Game/Tien/Blueprints/Interface/BPI_Enemy.SetFocus` _returnvalue (`/Game/Tien/Blueprints/AI/NewGen/AIC_Enemy_Base.ActorTarget` (`/Game/Tien/Characters/Enemy/BP_Enemy_Base.AIC Enemy Base` _asbp_enemy_base)))
      (return true))))

(fn `Received_NotifyEnd`
  (params (MeshComp :type "SkeletalMeshComponent Object Reference") (Animation :type "AnimSequenceBase Object Reference") (EventReference :type "AnimNotifyEventReference Structure (by ref)"))
  (returns (ReturnValue :type Boolean))
  (bind _returnvalue (`ActorComponent.GetOwner` MeshComp))
  (`/Engine/EditorBlueprintResources/StandardMacros.IsValid` _returnvalue
    (:`Is Valid`
      (message `/Game/Tien/Blueprints/Interface/BPI_Enemy.ClearFocus` _returnvalue)
      (return false))))