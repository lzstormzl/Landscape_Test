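; Base projectile Blueprint that moves at a configurable speed and gravity, applied to its movement component in the construction script.
; The box collision ignores the projectile's owner while moving.
; On hit, it broadcasts OnProjectileHit with the target and hit result, spawns a lightning slash impact Niagara effect, then destroys itself.
; A setter stores a DamageResponse, which is not used within this Blueprint's graphs.
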(event `self.ReceiveBeginPlay`
  (`PrimitiveComponent.IgnoreActorWhenMoving` (`self.BoxCollision`) (`self.GetOwner`) true))

(event `self.BoxCollision.OnComponentHit`
  (params (HitComponent :type "PrimitiveComponent Object Reference") (OtherActor :type "Actor Object Reference") (OtherComp :type "PrimitiveComponent Object Reference") (NormalImpulse :type "Vector Structure") (Hit :type "HitResult Structure (by ref)"))
  (`self.OnProjectileHit` OtherActor Hit)
  (`NiagaraFunctionLibrary.SpawnSystemAtLocation` "/Game/_SourcePackage/Hack_And_Slash_FX/VFX_Niagara/Impacts/NS_Lightning_Slash_Impact.NS_Lightning_Slash_Impact" (`.ImpactPoint` (`GameplayStatics.BreakHitResult` Hit)))
  (`self.K2_DestroyActor`))

(fn `SetProjectileHitResponse`
  (params (`Hit Response` :type "/Game/Tien/Blueprints/Enums/E_DamageResponse Enum" :default "NewEnumerator0"))
  (set `self.DamageResponse` `Hit Response`))

(fn `UserConstructionScript`
  (bind _projectilemovement (`self.ProjectileMovement`))
  (bind _projectilespeed (`self.ProjectileSpeed`))
  (set `ProjectileMovementComponent.InitialSpeed` _projectilespeed _projectilemovement)
  (set `ProjectileMovementComponent.MaxSpeed` _projectilespeed _projectilemovement)
  (set `ProjectileMovementComponent.ProjectileGravityScale` (`self.Gravity`) _projectilemovement))