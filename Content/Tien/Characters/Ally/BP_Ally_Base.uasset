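; Base character for AI-controlled allies, with optional timed lifespan that scales them in on possession and back out before expiry.
; Rotating turns it toward the controller's target using yaw timelines, then plays left, right or 180-degree montages.
; State setters drive the AIC_Ally_Base blackboard, movement flag and focus, while health, team and damage calls go to components.
; Includes helpers for montage lookup, hit tracking, sphere-trace hit prediction and hitstop; death destroys the actor.
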(event `Rotating`
  (bind _savedeltaz (`self.SaveDeltaZ`))
  (bind (_characterrotation_roll _characterrotation_pitch _characterrotation_yaw) (`KismetMathLibrary.BreakRotator` (`self.CharacterRotation`)))
  (bind (_characterrotation_roll_2 _characterrotation_pitch_2 _characterrotation_yaw_2) (`KismetMathLibrary.BreakRotator` (`self.CharacterRotation`)))
  (bind _savedeltaz_2 (`self.SaveDeltaZ`))
  (bind _actortarget (`/Game/Tien/Characters/Ally/AIC_Ally_Base.ActorTarget` (`self.AIC Ally Base`)))
  (bind _returnvalue (select `bool` (>= (`self.SaveDeltaZ`) 110.0) :`false` "/Game/Tien/Characters/Enemy/Chicken/Animations/AM_Boss_Ga_Rotate_Right.AM_Boss_Ga_Rotate_Right" :`true` "/Game/Tien/Characters/Enemy/Chicken/Animations/AM_Boss_Ga_Rotate180.AM_Boss_Ga_Rotate180" :!type "AnimMontage Object Reference"))
  (bind _returnvalue_2 (select `bool` (<= (`self.SaveDeltaZ`) -110.0) :`false` "/Game/Tien/Characters/Enemy/Chicken/Animations/AM_Boss_Ga_Rotate_Left.AM_Boss_Ga_Rotate_Left" :`true` "/Game/Tien/Characters/Enemy/Chicken/Animations/AM_Boss_Ga_Rotate180.AM_Boss_Ga_Rotate180" :!type "AnimMontage Object Reference"))
  (bind (_returnvalue_roll _returnvalue_pitch _returnvalue_yaw) (`KismetMathLibrary.BreakRotator` (`KismetMathLibrary.NormalizedDeltaRotator` (`KismetMathLibrary.FindLookAtRotation` (`self.K2_GetActorLocation`) (`self.K2_GetActorLocation` _actortarget)) (`self.CharacterRotation`))))
  (set `self.CharacterRotation` (`self.K2_GetActorRotation`))
  (`/Engine/EditorBlueprintResources/StandardMacros.IsValid` _actortarget
    (:`Is Valid`
      (bind _output_get (set `self.SaveDeltaZ` _returnvalue_yaw))
      (if (< _output_get 0.0)
        ;[1 0.4219 0.4219] Xoay Trái
        (bind (_direction _0_5 _0_64) (`Timeline|TurnInPlaceLeft` :!via `PlayFromStart`)
          (:`Update`
            (`self.K2_SetActorRotation` (`KismetMathLibrary.MakeRotator` _characterrotation_roll_2 _characterrotation_pitch_2 (`KismetMathLibrary.Lerp` _characterrotation_yaw_2 (+ _characterrotation_yaw_2 _savedeltaz) (`KismetMathLibrary.SelectFloat` _0_64 _0_5 (<= _savedeltaz -110.0)))))
            (`/Engine/EditorBlueprintResources/StandardMacros.DoOnce` false :!label _label
              (:`Completed`
                (if (== _returnvalue_2 "/Game/Tien/Characters/Enemy/Chicken/Animations/AM_Boss_Ga_Rotate_Left.AM_Boss_Ga_Rotate_Left")
                  (set `self.StartingPositionMontage` 0.67)
                  (else
                    (set `self.StartingPositionMontage` 0.38)))
                (`|PlayMontage` (`self.Mesh`) _returnvalue_2 1.0 (`self.StartingPositionMontage`)
                  (:`OnCompleted`
                    _)
                  (:`OnInterrupted`
                    _))
                (`self.OnRotateFinish`)
                (goto _label :!via `Reset`)))))
        (else
          ;[0.2458 0.2784 1] Xoay phải
          (bind (_direction_2 _0_89 _0_64_2) (`Timeline|TurnInPlaceRight` :!via `PlayFromStart`)
            (:`Update`
              (`self.K2_SetActorRotation` (`KismetMathLibrary.MakeRotator` _characterrotation_roll _characterrotation_pitch (`KismetMathLibrary.Lerp` _characterrotation_yaw (+ _characterrotation_yaw _savedeltaz_2) (`KismetMathLibrary.SelectFloat` _0_64_2 _0_89 (>= _savedeltaz_2 110.0)))))
              (`/Engine/EditorBlueprintResources/StandardMacros.DoOnce` false :!label _label_2
                (:`Completed`
                  (if (== _returnvalue "/Game/Tien/Characters/Enemy/Chicken/Animations/AM_Boss_Ga_Rotate_Right.AM_Boss_Ga_Rotate_Right")
                    (set `self.StartingPositionMontage` 0.16)
                    (else
                      (set `self.StartingPositionMontage` 0.38)))
                  (`|PlayMontage` (`self.Mesh`) _returnvalue 1.0 (`self.StartingPositionMontage`)
                    (:`OnCompleted`
                      _)
                    (:`OnInterrupted`
                      _))
                  (`self.OnRotateFinish`)
                  (goto _label_2 :!via `Reset`))))))))))

(event `self.ReceivePossessed`
  (params (NewController :type "Controller Object Reference"))
  (bind _lifespanvalue (`self.LifespanValue`))
  (`self.SetActorScale3D` (0.0 0.0 0.0))
  (`KismetSystemLibrary.Delay` 0.01)
  (if (not (<= _lifespanvalue 0.0))
    (`self.SetLifeSpan` _lifespanvalue)
    (bind (_direction _1) (`Timeline|TimeLine 0 - 1` :!via `PlayFromStart`)
      (:`Update`
        (`self.SetActorScale3D` (`KismetMathLibrary.Conv_DoubleToVector` _1))
        (`KismetSystemLibrary.Delay` (- _lifespanvalue 0.1))
        (`TimelineComponent.Reverse` (`self.TimeLine 0 - 1`))))))

(event `self.ReceiveBeginPlay`
  (bind _returnvalue (`GameplayStatics.GetActorOfClass` "/Game/Tien/Characters/Player/BP_ThuyTinhTien.BP_ThuyTinhTien_C"))
  (set `self.ThuyTinhRef` _returnvalue)
  (bind _asaic_ally_base (cast `/Game/Tien/Characters/Ally/AIC_Ally_Base` (`AIBlueprintHelperLibrary.GetAIController` self)))
  (set `self.AIC Ally Base` _asaic_ally_base))

(event `self.BPC_DamageSystem.OnDeath`
  (bind _mesh (`self.Mesh`))
  (`PrimitiveComponent.SetSimulatePhysics` _mesh true)
  (`PrimitiveComponent.SetCollisionEnabled` _mesh "QueryAndPhysics")
  (`self.K2_DestroyActor`))

(event `self.BPC_DamageSystem.OnDamagedResponse`
  (params (DamageResponse :type "/Game/Tien/Blueprints/Enums/E_DamageResponse Enum" :default "NewEnumerator0"))
  (switch `/Game/Tien/Blueprints/Enums/E_DamageResponse` DamageResponse))

(event `self.Attack`
  (params (AttackTarget :type "Actor Object Reference")))

(event `self.ClearDamagedActor`
  (`self.ClearDamagedActorArray`))

(event `self.SetFocus`
  (params (Target :type "Actor Object Reference"))
  (`self.SetFocusBase` Target))

(event `self.ClearFocus`
  (`self.ClearFocusBase`))

(event `self.BossUIActive.OnComponentBeginOverlap`
  (params (OverlappedComponent :type "PrimitiveComponent Object Reference") (OtherActor :type "Actor Object Reference") (OtherComp :type "PrimitiveComponent Object Reference") (OtherBodyIndex :type Integer) (bFromSweep :type Boolean) (SweepResult :type "HitResult Structure (by ref)")))

(fn `AddBoneName`
  (params (BoneName :type String))
  (`KismetArrayLibrary.Array_AddUnique` (`self.TraceBoneName`) BoneName))

(fn `AddDamageActorArray`
  (params (Actor :type "Actor Object Reference (by ref)"))
  (`KismetArrayLibrary.Array_AddUnique` (`self.HitActorArray`) Actor))

(fn `AOETraceSphere`
  (params (Location :type "Vector Structure") (AttackRange :type "Float (double-precision)"))
  (returns (HitActor :type "Actor Object Reference"))
  (bind (_outhit _returnvalue) (`KismetSystemLibrary.SphereTraceSingleForObjects` Location Location AttackRange (`|MakeArray` "ObjectTypeQuery3" :!type "EObjectTypeQuery Enum")))
  (if _returnvalue
    (return (`.HitActor` (`GameplayStatics.BreakHitResult` _outhit)))
    (else
      (return null))))

(fn `ClearBoneNameArray`
  (`KismetArrayLibrary.Array_Clear` (`self.TraceBoneName`)))

(fn `ClearDamagedActorArray`
  (`KismetArrayLibrary.Array_Clear` (`self.HitActorArray`)))

(fn `ClearFocusBase`
  (bind _aic_ally_base (`self.AIC Ally Base`))
  (bind _charactermovement (`self.CharacterMovement`))
  (set `CharacterMovementComponent.bOrientRotationToMovement` true _charactermovement)
  (set `CharacterMovementComponent.bUseControllerDesiredRotation` false _charactermovement)
  (`/Engine/EditorBlueprintResources/StandardMacros.IsValid` _aic_ally_base
    (:`Is Valid`
      (`AIController.K2_ClearFocus` _aic_ally_base))))

(fn `EndHitstop`
  (`GameplayStatics.SetGlobalTimeDilation` 1.0))

(fn `FindAttackMontage`
  (params (Combo :type Integer))
  (returns (Montage :type "AnimMontage Object Reference") (DamageResponse :type "/Game/Tien/Blueprints/Enums/E_DamageResponse Enum"))
  (bind _map_attackmontage (`self.Map_AttackMontage`))
  (bind _keys (`BlueprintMapLibrary.Map_Keys` _map_attackmontage))
  (for _array_element _keys
    (bind (_value _returnvalue) (`BlueprintMapLibrary.Map_Find` _map_attackmontage _array_element))
    (if _returnvalue
      (bind (_sortstring _thuytuongequip _damageresponse) (break `/Game/Tien/Blueprints/Struct/S_AttackMontage` _value))
      (if (`KismetStringLibrary.EqualEqual_StrStr` _sortstring (`KismetStringLibrary.Concat_StrStr` "Combo" (`KismetStringLibrary.Conv_IntToString` (`local.Combo`))))
        (`|ExecutionSequence`
          (:`then_0`
            (break))
          (:`then_1`
            (return _array_element _damageresponse))))
      (else
        (`KismetSystemLibrary.PrintString` "Không tìm thấy Attack Montage này!!")))))

(fn `GetAnimationLength`
  (params (Animation :type "AnimationAsset Object Reference"))
  (returns (Lenght :type "Float (double-precision)"))
  (return (`AnimationAsset.GetPlayLength` Animation)))

(fn `GetCurrentHealth`
  (returns (CurrentHealth :type "Float (double-precision)"))
  (return (`/Game/Tien/Blueprints/Components/BPC_StatsComponent.CurrentHealth` (`self.BPC_StatsComponent`))))

(fn `GetMaxHealth`
  (returns (MaxHealth :type "Float (double-precision)"))
  (return (`/Game/Tien/Blueprints/Components/BPC_StatsComponent.MaxHealth` (`self.BPC_StatsComponent`))))

(fn `GetMontageLength`
  (params (Montage :type "AnimMontage Object Reference"))
  (returns (Lenght :type "Float (double-precision)"))
  (return (`AnimationAsset.GetPlayLength` Montage)))

(fn `GetRef`
  (returns (Ref :type "Actor Object Reference"))
  (return self))

(fn `GetTeam`
  (returns (Team :type "/Game/Tien/Blueprints/Enums/E_Team Enum"))
  (return (`/Game/Tien/Blueprints/Components/BPC_TeamSystem.Team` (`self.BPC_TeamSystem`))))

(fn `IsActorHit?`
  (params (Actor :type "Actor Object Reference"))
  (returns (`IsContain?` :type Boolean))
  (return (`KismetArrayLibrary.Array_Contains` (`self.HitActorArray`) Actor)))

(fn `IsTeam`
  (params (CompareTeam :type "/Game/Tien/Blueprints/Enums/E_Team Enum" :default "NewEnumerator0"))
  (returns (IsTeam :type Boolean))
  (bind _teamup (`/Game/Tien/Blueprints/Components/BPC_TeamSystem.IsTeam` (`self.BPC_TeamSystem`) CompareTeam))
  (return _teamup))

(fn `SetCharacterState`
  (params (CharacterState :type "/Game/Tien/Blueprints/Enums/E_CharacterState Enum" :default "NewEnumerator0"))
  (switch `/Game/Tien/Blueprints/Enums/E_CharacterState` CharacterState
    (:`NewEnumerator0`
      (`self.SetCharacterStateAsIdle`))
    (:`NewEnumerator3`
      (`self.SetCharacterStateAsStuning`))
    (:`NewEnumerator4`
      (`self.SetCharacterStateAsFalling`))))

(fn `SetCharacterStateAsFalling`
  (bind _aic_ally_base (`self.AIC Ally Base`))
  (bind _output_get (set `self.CurrentCharacterState` "NewEnumerator4"))
  (`BlackboardComponent.SetValueAsEnum` (`AIController.Blackboard` _aic_ally_base) (`/Game/Tien/Characters/Ally/AIC_Ally_Base.CharacterStatesKeyName` _aic_ally_base) _output_get)
  (set `self.CanMove?` false)
  (`AIController.K2_ClearFocus` _aic_ally_base))

(fn `SetCharacterStateAsIdle`
  (bind _aic_ally_base (`self.AIC Ally Base`))
  (bind _output_get (set `self.CurrentCharacterState` "NewEnumerator0"))
  (`BlackboardComponent.SetValueAsEnum` (`AIController.Blackboard` _aic_ally_base) (`/Game/Tien/Characters/Ally/AIC_Ally_Base.CharacterStatesKeyName` _aic_ally_base) _output_get)
  (set `self.CanMove?` true))

(fn `SetCharacterStateAsStuning`
  (bind _aic_ally_base (`self.AIC Ally Base`))
  (bind _output_get (set `self.CurrentCharacterState` "NewEnumerator3"))
  (`BlackboardComponent.SetValueAsEnum` (`AIController.Blackboard` _aic_ally_base) (`/Game/Tien/Characters/Ally/AIC_Ally_Base.CharacterStatesKeyName` _aic_ally_base) _output_get)
  (set `self.CanMove?` false)
  (`AIController.K2_ClearFocus` _aic_ally_base))

(fn `SetFocusBase`
  (params (FocusTarget :type "Actor Object Reference"))
  (bind _charactermovement (`self.CharacterMovement`))
  (set `CharacterMovementComponent.bOrientRotationToMovement` false _charactermovement)
  (set `CharacterMovementComponent.bUseControllerDesiredRotation` true _charactermovement)
  (`AIController.K2_SetFocus` (`self.AIC Ally Base`) FocusTarget))

(fn `SetMovementSpeed`
  (params (MovementSpeed :type "/Game/Tien/Blueprints/Enums/E_MovementSpeed Enum" :default "NewEnumerator0"))
  (returns (Speed :type "Float (double-precision)"))
  (bind _output_get (set `CharacterMovementComponent.MaxWalkSpeed` (select `/Game/Tien/Blueprints/Enums/E_MovementSpeed` MovementSpeed :`NewEnumerator1` 150.0 :`NewEnumerator2` 350.0 :`NewEnumerator3` 1200.0 :!type "Float (single-precision)") (`self.CharacterMovement`)))
  (return _output_get))

(fn `SetTeam`
  (params (Team :type "/Game/Tien/Blueprints/Enums/E_Team Enum" :default "NewEnumerator0"))
  (returns (NewTeam :type "/Game/Tien/Blueprints/Enums/E_Team Enum"))
  (bind _newteam (`/Game/Tien/Blueprints/Components/BPC_TeamSystem.SetTeam` (`self.BPC_TeamSystem`) Team))
  (return _newteam))

(fn `StartHitstop`
  (params (Value :type "Float (double-precision)"))
  (`GameplayStatics.SetGlobalTimeDilation` 0.1)
  (`KismetSystemLibrary.K2_SetTimer` null "EndHitstop" Value true))

(fn `TakeDamage`
  (params (DamageInfo :type "/Game/Tien/Blueprints/Struct/S_DamageInfo Structure"))
  (returns (IsDamaged :type Boolean))
  (bind _isdamaged (`/Game/Tien/Blueprints/Components/BPC_DamageSystem.TakeDamage` (`self.BPC_DamageSystem`) DamageInfo))
  (return _isdamaged))

(fn `UserConstructionScript`)

(fn `WillHit`
  (params (ActorToHit :type "Actor Object Reference"))
  (returns (`WasHit?` :type Boolean))
  (bind (_currentattackinfo_starttime _currentattackinfo_duration) (break `/Game/Tien/Blueprints/Struct/S_AttackInfo` (`self.CurrentAttackInfo`)))
  (bind _attackrange (`self.AttackRange`))
  (bind _hitactor (`self.AOETraceSphere` (+ (`self.K2_GetActorLocation`) (* (`self.GetActorForwardVector`) (* (/ (- (+ _currentattackinfo_starttime _currentattackinfo_duration) _currentattackinfo_starttime) _currentattackinfo_duration) _attackrange))) _attackrange))
  (return (== _hitactor (`local.ActorToHit`))))