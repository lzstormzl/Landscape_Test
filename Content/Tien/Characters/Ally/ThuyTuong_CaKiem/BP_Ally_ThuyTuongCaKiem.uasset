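; Ally character ThuyTuongCaKiem, a child Blueprint that provides two melee attacks.
; Attack and Attack2 play their montages, set combo damage and response, and signal attack finish on completion or interruption.
; Start and end trace events toggle a fast looping timer that sphere-traces at the right-hand socket.
; Traces skip teammates and already-hit actors, send damage through a message, and spawn a splash effect when it succeeds.
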(event `/Game/Tien/Blueprints/Interface/BPI_TraceDamage.EndTraceDamage1`
  (`KismetSystemLibrary.K2_ClearAndInvalidateTimerHandle` (stale `/Game/Tien/Blueprints/Interface/BPI_TraceDamage.StartTraceDamge1` _returnvalue)))

(event `/Game/Tien/Blueprints/Interface/BPI_TraceDamage.StartTraceDamge1`
  (bind _returnvalue (`KismetSystemLibrary.K2_SetTimerDelegate` (delegate `TraceDamage1`) 0.01 true)))

(event `TraceDamage1`
  (bind _mesh (`self.Mesh`))
  (bind (_outhit _returnvalue) (`KismetSystemLibrary.SphereTraceSingleForObjects` (`SceneComponent.GetSocketLocation` _mesh "RightHandMiddle1") (`SceneComponent.GetSocketLocation` _mesh "RightHandMiddle1") 50.0 (`|MakeArray` "ObjectTypeQuery3" :!type "EObjectTypeQuery Enum")))
  (if _returnvalue
    (bind (_bblockinghit _binitialoverlap _time _distance _location _impactpoint _normal _impactnormal _physmat _hitactor) (`GameplayStatics.BreakHitResult` _outhit))
    (bind _iscontain_ (`self.IsActorHit?` _hitactor))
    (bind _isteam (message `/Game/Tien/Blueprints/Interface/BPI_Team.IsTeam` _hitactor "NewEnumerator2"))
    (if (not (or _isteam _iscontain_))
      (`self.AddDamageActorArray` _hitactor)
      (bind _isdamaged (message `/Game/Tien/Blueprints/Interface/BPI_Damgable.TakeDamage` _hitactor (make `/Game/Tien/Blueprints/Struct/S_DamageInfo` (`self.DamageCombo`) "NewEnumerator0" (`self.DamageResponse`))))
      (if _isdamaged
        (`NiagaraFunctionLibrary.SpawnSystemAtLocation` "/Game/_SourcePackage/_Blood_VFX_Pack/Particles/Systems/P_BigSplash_Hit.P_BigSplash_Hit" _impactpoint)))))

(event `/Game/Tien/Blueprints/Interface/BPI_Enemy.Attack`
  (params (AttackTarget :type "Actor Object Reference"))
  (`|PlayMontage` (`self.Mesh`) "/Game/Tien/Characters/Ally/ThuyTuong_CaKiem/Animations/TTg_CaKiem_Atk1_Montage.TTg_CaKiem_Atk1_Montage"
    (:`then`
      (set `self.DamageResponse` "NewEnumerator3")
      (set `self.DamageCombo` 10.0))
    (:`OnCompleted`
      (`self.OnAttackFinish` :!label _label))
    (:`OnInterrupted`
      (goto _label))))

(event `/Game/Tien/Blueprints/Interface/BPI_Enemy.Attack 2`
  (params (AttackTarget :type "Actor Object Reference"))
  (`|PlayMontage` (`self.Mesh`) "/Game/Tien/Characters/Ally/ThuyTuong_CaKiem/Animations/TTg_CaKiem_Atk2_Montage.TTg_CaKiem_Atk2_Montage"
    (:`then`
      (set `self.DamageResponse` "NewEnumerator3")
      (set `self.DamageCombo` 10.0))
    (:`OnCompleted`
      (`self.OnAttackFinish` :!label _label_2))
    (:`OnInterrupted`
      (goto _label_2))))

(fn `UserConstructionScript`
  (`parent.UserConstructionScript`))