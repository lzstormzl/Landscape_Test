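; Spear-wielding enemy character that spawns a spear on its hand socket and destroys it on death.
; Its attack chains two montages, the second slower and heavier-hitting, signaling attack finish when the second completes or is interrupted.
; Start/end trace events run a looping timer that sphere-traces pawns between spear sockets.
; New hit actors are recorded, sent damage through an interface message, and show a splash effect when damaged.
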(event `self.ReceiveBeginPlay`
  (`parent.ReceiveBeginPlay`)
  (bind _returnvalue (`|SpawnActorFromClass` "/Game/Tien/Characters/Enemy/Spear/Weapon/BP_Spear.BP_Spear_C" (`SceneComponent.GetSocketTransform` (`self.Mesh`) "hand_rSpear" "RTS_World") "Undefined" "MultiplyWithRoot" null null))
  (bind _output_get (set `self.SpearRef` _returnvalue))
  (`self.K2_AttachToComponent` _output_get (`self.Mesh`) "hand_rSpear" "SnapToTarget" "SnapToTarget" "SnapToTarget" true))

(event `/Game/Tien/Blueprints/Interface/BPI_Enemy.Attack`
  (params (AttackTarget :type "Actor Object Reference"))
  (`|PlayMontage` (`self.Mesh`) "/Game/Tien/Characters/Enemy/Spear/Animation/AM_Spear_Combo02_2_Montage.AM_Spear_Combo02_2_Montage"
    (:`then`
      (set `self.DamageResponse` "NewEnumerator2")
      (set `self.DamageCombo` 1.0))
    (:`OnCompleted`
      (`|PlayMontage` (`self.Mesh`) "/Game/Tien/Characters/Enemy/Spear/Animation/AM_Spear_Combo02_3_Montage.AM_Spear_Combo02_3_Montage" 0.5
        (:`then`
          (set `self.DamageResponse` "NewEnumerator3")
          (set `self.DamageCombo` 3.0))
        (:`OnCompleted`
          (`self.OnAttackFinish` :!label _label))
        (:`OnInterrupted`
          (goto _label))))))

(event `self.BPC_DamageSystem.OnDeath`
  (`self.K2_DestroyActor` (`self.SpearRef`)))

(event `self.BPC_DamageSystem.OnDamagedResponse`
  (params (DamageResponse :type "/Game/Tien/Blueprints/Enums/E_DamageResponse Enum" :default "NewEnumerator0")))

(event `/Game/Tien/Blueprints/Interface/BPI_TraceDamage.EndTraceDamage1`
  (`KismetSystemLibrary.K2_ClearAndInvalidateTimerHandle` (stale `/Game/Tien/Blueprints/Interface/BPI_TraceDamage.StartTraceDamge1` _returnvalue)))

(event `/Game/Tien/Blueprints/Interface/BPI_TraceDamage.StartTraceDamge1`
  (bind _returnvalue (`KismetSystemLibrary.K2_SetTimerDelegate` (delegate `TraceDamage1`) 0.01 true)))

(event `TraceDamage1`
  (bind _mesh (`self.Mesh`))
  (bind (_outhit _returnvalue) (`KismetSystemLibrary.SphereTraceSingleForObjects` (`SceneComponent.GetSocketLocation` _mesh "StartSpear") (`SceneComponent.GetSocketLocation` _mesh "EndSpear") 50.0 (`|MakeArray` "ObjectTypeQuery3" :!type "EObjectTypeQuery Enum")))
  (if _returnvalue
    (bind (_bblockinghit _binitialoverlap _time _distance _location _impactpoint _normal _impactnormal _physmat _hitactor) (`GameplayStatics.BreakHitResult` _outhit))
    (bind _iscontain_ (`self.IsActorHit?` _hitactor))
    (if (not _iscontain_)
      (`self.AddDamageActorArray` _hitactor)
      (bind _isdamaged (message `/Game/Tien/Blueprints/Interface/BPI_Damgable.TakeDamage` _hitactor (make `/Game/Tien/Blueprints/Struct/S_DamageInfo` (`self.DamageCombo`) "NewEnumerator0" (`self.DamageResponse`))))
      (if _isdamaged
        (`NiagaraFunctionLibrary.SpawnSystemAtLocation` "/Game/_SourcePackage/_Blood_VFX_Pack/Particles/Systems/P_BigSplash_Hit.P_BigSplash_Hit" _impactpoint)))))

(fn `FindAttackMontage`
  (params (Combo :type Integer))
  (returns (Montage :type "AnimMontage Object Reference") (DamageResponse :type "/Game/Tien/Blueprints/Enums/E_DamageResponse Enum"))
  (bind (_montage _damageresponse) (`parent.FindAttackMontage` Combo))
  (return _montage _damageresponse))

(fn `GetRef`
  (returns (Ref :type "Actor Object Reference"))
  (return self))

(fn `TakeDamage`
  (params (DamageInfo :type "/Game/Tien/Blueprints/Struct/S_DamageInfo Structure"))
  (returns (IsDamaged :type Boolean))
  (bind _isdamaged (`/Game/Tien/Blueprints/Components/BPC_DamageSystem.TakeDamage` (`self.BPC_DamageSystem`) DamageInfo))
  (return _isdamaged))

(fn `UserConstructionScript`
  (`parent.UserConstructionScript`))