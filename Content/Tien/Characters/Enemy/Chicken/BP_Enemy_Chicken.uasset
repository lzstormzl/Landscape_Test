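; Chicken boss enemy Blueprint with three standard montage attacks and a motion-warped leap at the AI target that also animates the player camera's FOV.
; Each attack sets damage, a Falling response and hit bones, and disables interruption until it ends.
; A looping timer sphere-traces up to three bone sockets, damaging each actor once and spawning splash effects.
; Taking Falling damage plays a hit react with camera shake and state changes.
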(event `/Game/Tien/Blueprints/Interface/BPI_Enemy.Attack`
  (params (AttackTarget :type "Actor Object Reference"))
  (bind _bpc_damagesystem (`self.BPC_DamageSystem`))
  (`|PlayMontage` (`self.Mesh`) "/Game/Tien/Characters/Enemy/Chicken/Animations/Boss_Ga_Attack_Anim_Montage.Boss_Ga_Attack_Anim_Montage" 1.5
    (:`then`
      (set `/Game/Tien/Blueprints/Components/BPC_DamageSystem.IsInterruptible` false _bpc_damagesystem)
      (set `self.DamageCombo` 30.0)
      (set `self.DamageResponse` "NewEnumerator3")
      (`self.AddBoneName` "Jaw")
      (`self.AddBoneName` "Right_Foot"))
    (:`OnCompleted`
      (`self.ClearBoneNameArray` :!label _label)
      (`self.OnAttackFinish`)
      (set `/Game/Tien/Blueprints/Components/BPC_DamageSystem.IsInterruptible` true _bpc_damagesystem))
    (:`OnInterrupted`
      (goto _label))))

(event `/Game/Tien/Blueprints/Interface/BPI_Enemy.Attack 2`
  (params (AttackTarget :type "Actor Object Reference"))
  (bind _bpc_damagesystem (`self.BPC_DamageSystem`))
  (`|PlayMontage` (`self.Mesh`) "/Game/Tien/Characters/Enemy/Chicken/Animations/Boss_Ga_Attack2_Anim_Montage.Boss_Ga_Attack2_Anim_Montage" 1.5
    (:`then`
      (set `/Game/Tien/Blueprints/Components/BPC_DamageSystem.IsInterruptible` false _bpc_damagesystem)
      (set `self.DamageCombo` 30.0)
      (set `self.DamageResponse` "NewEnumerator3")
      (`self.AddBoneName` "Right_Foot"))
    (:`OnCompleted`
      (`self.OnAttackFinish` :!label _label_2)
      (`self.ClearBoneNameArray`)
      (set `/Game/Tien/Blueprints/Components/BPC_DamageSystem.IsInterruptible` true _bpc_damagesystem))
    (:`OnInterrupted`
      (goto _label_2))))

(event `/Game/Tien/Blueprints/Interface/BPI_Enemy.Attack 3`
  (params (AttackTarget :type "Actor Object Reference"))
  (bind _bpc_damagesystem (`self.BPC_DamageSystem`))
  (`|PlayMontage` (`self.Mesh`) "/Game/Tien/Characters/Enemy/Chicken/Animations/Boss_Ga_Attack4_Anim_Montage.Boss_Ga_Attack4_Anim_Montage"
    (:`then`
      (set `/Game/Tien/Blueprints/Components/BPC_DamageSystem.IsInterruptible` false _bpc_damagesystem)
      (set `self.DamageCombo` 30.0)
      (set `self.DamageResponse` "NewEnumerator3")
      (`self.AddBoneName` "Jaw"))
    (:`OnCompleted`
      (`self.OnAttackFinish` :!label _label_3)
      (`self.ClearBoneNameArray`)
      (set `/Game/Tien/Blueprints/Components/BPC_DamageSystem.IsInterruptible` true _bpc_damagesystem))
    (:`OnInterrupted`
      (goto _label_3))))

(event `ChickenLeapAttack`
  (bind _bpc_damagesystem (`self.BPC_DamageSystem`))
  (bind _actortarget (`/Game/Tien/Blueprints/AI/NewGen/AIC_Enemy_Base.ActorTarget` (`self.AIC Enemy Base`)))
  (bind _returnvalue (`self.K2_GetActorLocation` _actortarget))
  (bind _notifyname (`|PlayMontage` (`self.Mesh`) "/Game/Tien/Characters/Enemy/Chicken/Animations/Boss_Ga_Attack_3_Anim_Montage.Boss_Ga_Attack_3_Anim_Montage")
    (:`then`
      (set `/Game/Tien/Blueprints/Components/BPC_DamageSystem.IsInterruptible` false _bpc_damagesystem)
      (set `self.DamageCombo` 30.0)
      (set `self.DamageResponse` "NewEnumerator3")
      (`self.AddBoneName` "Left_Foot")
      (`self.AddBoneName` "Right_Foot")
      (`self.AddBoneName` "Jaw")
      (bind (_direction _start) (`Timeline|StartFieldOfView` :!via `PlayFromStart`)
        (:`Update`
          (`CameraComponent.SetFieldOfView` (`/Game/Tien/Characters/Player/BP_ThuyTinhTien.FollowCamera` (`self.ThuyTinhRef`)) _start))))
    (:`OnCompleted`
      (`self.OnAttackFinish` :!label _label_4)
      (`MotionWarpingComponent.RemoveWarpTarget` (`self.MotionWarping`) "leapattack")
      (`self.ClearBoneNameArray`)
      (set `/Game/Tien/Blueprints/Components/BPC_DamageSystem.IsInterruptible` true _bpc_damagesystem)
      (bind (_direction_2 _start_2) (`Timeline|Timeline_0` :!via `PlayFromStart`)
        (:`Update`
          (`CameraComponent.SetFieldOfView` (`/Game/Tien/Characters/Player/BP_ThuyTinhTien.FollowCamera` (`self.ThuyTinhRef`)) _start_2))))
    (:`OnInterrupted`
      (goto _label_4))
    (:`OnNotifyBegin`
      (switch `name` _notifyname
        (:`ClearFocus`
          (`/Engine/EditorBlueprintResources/StandardMacros.IsValid` _actortarget
            (:`Is Valid`
              (`MotionWarpingComponent.AddOrUpdateWarpTarget` (`self.MotionWarping`) (make `MotionWarpingTarget` "leapattack" _returnvalue (`KismetMathLibrary.FindLookAtRotation` (`self.K2_GetActorLocation`) _returnvalue))))))))))

(event `WaitRotate`
  (`|PlayMontage` (`self.Mesh`)
    (:`OnCompleted`
      _)
    (:`OnInterrupted`
      _))
  (`self.OnAttackFinish`))

(event `/Game/Tien/Blueprints/Interface/BPI_TraceDamage.EndTraceDamage1`
  (`KismetSystemLibrary.K2_ClearAndInvalidateTimerHandle` (stale `/Game/Tien/Blueprints/Interface/BPI_TraceDamage.StartTraceDamge1` _returnvalue)))

(event `/Game/Tien/Blueprints/Interface/BPI_TraceDamage.StartTraceDamge1`
  (bind _returnvalue (`KismetSystemLibrary.K2_SetTimerDelegate` (delegate `TraceDamage1`) 0.0001 true)))

(event `TraceDamage1`
  (bind _returnvalue (`SceneComponent.GetSocketLocation` (`self.Mesh`) (`KismetStringLibrary.Conv_StringToName` (`|GetArrayItem` (`self.TraceBoneName`) 1))))
  (bind _returnvalue_2 (`SceneComponent.GetSocketLocation` (`self.Mesh`) (`KismetStringLibrary.Conv_StringToName` (`|GetArrayItem` (`self.TraceBoneName`) 2))))
  (bind _returnvalue_3 (`SceneComponent.GetSocketLocation` (`self.Mesh`) (`KismetStringLibrary.Conv_StringToName` (`|GetArrayItem` (`self.TraceBoneName`)))))
  (`|ExecutionSequence`
    (:`then_0`
      (bind (_outhit _returnvalue_4) (`KismetSystemLibrary.SphereTraceSingleForObjects` :`Start` _returnvalue_3 :`End` _returnvalue_3 :`Radius` 100.0 :`ObjectTypes` (`|MakeArray` "ObjectTypeQuery3" :!type "EObjectTypeQuery Enum") :`TraceColor` (struct :`R` 1.0 :`G` 1.0 :`B` 1.0 :`A` 1.0) :`TraceHitColor` (struct :`R` 1.0 :`G` 0.039115 :`A` 1.0)))
      (if _returnvalue_4
        (bind (_bblockinghit _binitialoverlap _time _distance _location _impactpoint _normal _impactnormal _physmat _hitactor) (`GameplayStatics.BreakHitResult` _outhit))
        ;[1 1 1] Gây sát thương 1 lần trên 1 đòn đánh
        (bind _iscontain_ (`self.IsActorHit?` _hitactor))
        (if (not _iscontain_)
          (`self.AddDamageActorArray` _hitactor)
          (bind _isdamaged (message `/Game/Tien/Blueprints/Interface/BPI_Damgable.TakeDamage` _hitactor (make `/Game/Tien/Blueprints/Struct/S_DamageInfo` (`self.DamageCombo`) "NewEnumerator0" (`self.DamageResponse`))))
          (if _isdamaged
            (`NiagaraFunctionLibrary.SpawnSystemAtLocation` "/Game/_SourcePackage/_Blood_VFX_Pack/Particles/Systems/P_BigSplash_Hit.P_BigSplash_Hit" _impactpoint)))))
    (:`then_1`
      (bind (_outhit_2 _returnvalue_5) (`KismetSystemLibrary.SphereTraceSingleForObjects` :`Start` _returnvalue :`End` _returnvalue :`Radius` 100.0 :`ObjectTypes` (`|MakeArray` "ObjectTypeQuery3" :!type "EObjectTypeQuery Enum") :`TraceColor` (struct :`R` 1.0 :`G` 1.0 :`B` 1.0 :`A` 1.0) :`TraceHitColor` (struct :`R` 1.0 :`G` 0.039115 :`A` 1.0)))
      (if _returnvalue_5
        (bind (_bblockinghit_2 _binitialoverlap_2 _time_2 _distance_2 _location_2 _impactpoint_2 _normal_2 _impactnormal_2 _physmat_2 _hitactor_2) (`GameplayStatics.BreakHitResult` _outhit_2))
        ;[1 1 1] Gây sát thương 1 lần trên 1 đòn đánh
        (bind _iscontain__2 (`self.IsActorHit?` _hitactor_2))
        (if (not _iscontain__2)
          (`self.AddDamageActorArray` _hitactor_2)
          (bind _isdamaged_2 (message `/Game/Tien/Blueprints/Interface/BPI_Damgable.TakeDamage` _hitactor_2 (make `/Game/Tien/Blueprints/Struct/S_DamageInfo` (`self.DamageCombo`) "NewEnumerator0" (`self.DamageResponse`))))
          (if _isdamaged_2
            (`NiagaraFunctionLibrary.SpawnSystemAtLocation` "/Game/_SourcePackage/_Blood_VFX_Pack/Particles/Systems/P_BigSplash_Hit.P_BigSplash_Hit" _impactpoint_2)))))
    (:`then_2`
      (bind (_outhit_3 _returnvalue_6) (`KismetSystemLibrary.SphereTraceSingleForObjects` :`Start` _returnvalue_2 :`End` _returnvalue_2 :`Radius` 100.0 :`ObjectTypes` (`|MakeArray` "ObjectTypeQuery3" :!type "EObjectTypeQuery Enum") :`TraceColor` (struct :`R` 1.0 :`G` 1.0 :`B` 1.0 :`A` 1.0) :`TraceHitColor` (struct :`R` 1.0 :`G` 0.039115 :`A` 1.0)))
      (if _returnvalue_6
        (bind (_bblockinghit_3 _binitialoverlap_3 _time_3 _distance_3 _location_3 _impactpoint_3 _normal_3 _impactnormal_3 _physmat_3 _hitactor_3) (`GameplayStatics.BreakHitResult` _outhit_3))
        ;[1 1 1] Gây sát thương 1 lần trên 1 đòn đánh
        (bind _iscontain__3 (`self.IsActorHit?` _hitactor_3))
        (if (not _iscontain__3)
          (`self.AddDamageActorArray` _hitactor_3)
          (bind _isdamaged_3 (message `/Game/Tien/Blueprints/Interface/BPI_Damgable.TakeDamage` _hitactor_3 (make `/Game/Tien/Blueprints/Struct/S_DamageInfo` (`self.DamageCombo`) "NewEnumerator0" (`self.DamageResponse`))))
          (if _isdamaged_3
            (`NiagaraFunctionLibrary.SpawnSystemAtLocation` "/Game/_SourcePackage/_Blood_VFX_Pack/Particles/Systems/P_BigSplash_Hit.P_BigSplash_Hit" _impactpoint_3)))))))

(event `self.BPC_DamageSystem.OnDamagedResponse`
  (params (DamageResponse :type "/Game/Tien/Blueprints/Enums/E_DamageResponse Enum" :default "NewEnumerator0"))
  (switch `/Game/Tien/Blueprints/Enums/E_DamageResponse` DamageResponse
    (:`NewEnumerator3`
      (`|PlayMontage` (`self.Mesh`) "/Game/Tien/Characters/Enemy/Chicken/Animations/Boss_Ga_HitReact_Right_Montage.Boss_Ga_HitReact_Right_Montage"
        (:`then`
          (`self.SetCharacterState` "NewEnumerator4")
          (set `self.IsFalling?` true)
          (`LegacyCameraShake.StartLegacyCameraShake` (`GameplayStatics.GetPlayerCameraManager` 0) "/Game/_SourcePackage/AEO_Abilities/Other/Sequencer/CameraShake.CameraShake_C" 13.0 "UserDefined")
          (`KismetSystemLibrary.PrintString` "Hello"))
        (:`OnCompleted`
          (set `self.IsFalling?` false)
          (bind _lenght (`self.GetAnimationLength` "/Game/Tien/Characters/Enemy/SwordAndShield/Animation/HitReaction/SworldShield_Getup.SworldShield_Getup"))
          (`KismetSystemLibrary.Delay` _lenght)
          (`self.SetCharacterState` "NewEnumerator0"))))))

(fn `UserConstructionScript`
  (`parent.UserConstructionScript`))