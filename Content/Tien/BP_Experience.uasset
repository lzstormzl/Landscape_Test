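; BP_Experience is a pickup that homes in on the player and calls a stamina-gain message on overlap.
; A timeline started at BeginPlay ramps the projectile movement's homing acceleration, aimed at the player character.
; Tick feeds the box location and current acceleration to Niagara parameters for the visual effect.
; Box overlap with a Player-tagged actor sends the message and sets a short lifespan rather than destroying immediately.
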(event `self.ReceiveBeginPlay`
  (set `ProjectileMovementComponent.HomingTargetComponent` (`Actor.RootComponent` (`GameplayStatics.GetPlayerCharacter` 0)) (`self.ProjectileMovement`))
  (bind (_direction _newtrack_0) (`Timeline|Timeline`)
    (:`Update`
      (set `ProjectileMovementComponent.HomingAccelerationMagnitude` (`KismetMathLibrary.Lerp` 1.0 10000.0 _newtrack_0) (`self.ProjectileMovement`)))))

(event `self.ReceiveTick`
  (params (DeltaSeconds :type "Float (single-precision)"))
  (`NiagaraComponent.SetVariableVec3` (`self.Niagara`) "StartHeight" (`SceneComponent.K2_GetComponentLocation` (`self.Box`)))
  (`NiagaraComponent.SetVariableFloat` (`self.Niagara`) "SpeedAttraction" (`ProjectileMovementComponent.HomingAccelerationMagnitude` (`self.ProjectileMovement`))))

(event `self.Box.OnComponentBeginOverlap`
  (params (OverlappedComponent :type "PrimitiveComponent Object Reference") (OtherActor :type "Actor Object Reference") (OtherComp :type "PrimitiveComponent Object Reference") (OtherBodyIndex :type Integer) (bFromSweep :type Boolean) (SweepResult :type "HitResult Structure (by ref)"))
  (if (`self.ActorHasTag` OtherActor "Player")
    (message `/Game/Tien/Blueprints/Interface/BPI_Stats.PlusStamina` OtherActor 2.0)
    (`self.SetLifeSpan` 1.0)))

(fn `UserConstructionScript`)