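; BP_ImposterB_E is the Imposter Beast boss enemy that fights the BP_Maze_Long player.
; Each tick it tracks the player, interpolating yaw while moving or playing turn montages when nearly stationary.
; Attack, jump, backstep and roar events play montages and signal animation end; limb hitboxes apply flag-gated damage unless the player dodges.
; It also flags a perfect-dodge radius, manages health, regen and death, and updates a boss health widget.
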(event `self.ReceiveTick`
  (params (DeltaSeconds :type "Float (single-precision)"))
  (`|ExecutionSequence`
    (:`then_0`
      (`self.FocusonPlayer`))
    (:`then_1`
      (bind _asbp_maze_long (cast `/Game/_MazeLong/BP_Maze_Long` (`GameplayStatics.GetPlayerCharacter` 0)))
      (set `self.PlayerDodging?` (`/Game/_MazeLong/BP_Maze_Long.Dodging` _asbp_maze_long)))))

(event `self.ReceiveBeginPlay`
  (`|ExecutionSequence`
    (:`then_0`
      (set `self.Lock Target` (`GameplayStatics.GetPlayerPawn` 0)))
    (:`then_1`
      (set `self.IsTurning` false))
    (:`then_2`
      (set `self.DamagedPlayer?` false)
      (set `self.ANS_Damage?` false))
    (:`then_3`
      (`|ExecutionSequence`
        (:`then_0`
          (bind _output_get (set `self.MaxHealth` 1500.0))
          (set `self.CurrentHealth` _output_get)
          (set `self.Death?` false)
          (set `self.HealthRegen` 8.0))
        (:`then_1`
          (bind _returnvalue (`|CreateWidget` "/Game/_MazeLong/_System/MazeLong_Info_Bar.MazeLong_Info_Bar_C" (`GameplayStatics.GetPlayerController` 0)))
          (bind _output_get_2 (set `self.UI_Info` _returnvalue))
          (`UserWidget.AddToViewport` _output_get_2 0))))))

(event `self.RHandHitBox.OnComponentBeginOverlap`
  (params (OverlappedComponent :type "PrimitiveComponent Object Reference") (OtherActor :type "Actor Object Reference") (OtherComp :type "PrimitiveComponent Object Reference") (OtherBodyIndex :type Integer) (bFromSweep :type Boolean) (SweepResult :type "HitResult Structure (by ref)"))
  (`self.MeleeHitBox` OtherActor))

(event `self.LHandHitBox.OnComponentBeginOverlap`
  (params (OverlappedComponent :type "PrimitiveComponent Object Reference") (OtherActor :type "Actor Object Reference") (OtherComp :type "PrimitiveComponent Object Reference") (OtherBodyIndex :type Integer) (bFromSweep :type Boolean) (SweepResult :type "HitResult Structure (by ref)"))
  (`self.MeleeHitBox` OtherActor))

(event `self.LLegHitBox.OnComponentBeginOverlap`
  (params (OverlappedComponent :type "PrimitiveComponent Object Reference") (OtherActor :type "Actor Object Reference") (OtherComp :type "PrimitiveComponent Object Reference") (OtherBodyIndex :type Integer) (bFromSweep :type Boolean) (SweepResult :type "HitResult Structure (by ref)"))
  (`self.MeleeHitBox` OtherActor))

(event `self.RLegHitBox.OnComponentBeginOverlap`
  (params (OverlappedComponent :type "PrimitiveComponent Object Reference") (OtherActor :type "Actor Object Reference") (OtherComp :type "PrimitiveComponent Object Reference") (OtherBodyIndex :type Integer) (bFromSweep :type Boolean) (SweepResult :type "HitResult Structure (by ref)"))
  (`self.MeleeHitBox` OtherActor))

(event `MeleeHitBox`
  (params (OtherActor :type "Actor Object Reference"))
  (if (and (`self.ANS_Damage?`) (not (`self.DamagedPlayer?`)) (not (`self.PlayerDodging?`)))
    (bind _asbp_maze_long (cast `/Game/_MazeLong/BP_Maze_Long` OtherActor))
    (`GameplayStatics.ApplyDamage` _asbp_maze_long 40.0)
    (set `self.DamagedPlayer?` true)))

(event `self.PerfectDodge_Radius.OnComponentBeginOverlap`
  (params (OverlappedComponent :type "PrimitiveComponent Object Reference") (OtherActor :type "Actor Object Reference") (OtherComp :type "PrimitiveComponent Object Reference") (OtherBodyIndex :type Integer) (bFromSweep :type Boolean) (SweepResult :type "HitResult Structure (by ref)"))
  (cast `/Game/_MazeLong/BP_Maze_Long` OtherActor)
  (set `self.PerfectDodgeRadius?` true))

(event `self.PerfectDodge_Radius.OnComponentEndOverlap`
  (params (OverlappedComponent :type "PrimitiveComponent Object Reference") (OtherActor :type "Actor Object Reference") (OtherComp :type "PrimitiveComponent Object Reference") (OtherBodyIndex :type Integer))
  (cast `/Game/_MazeLong/BP_Maze_Long` OtherActor)
  (set `self.PerfectDodgeRadius?` false))

(event `FocusonPlayer`
  (bind _returnvalue (`self.K2_GetActorRotation`))
  (bind _lock_target (`self.Lock Target`)
    (:`then`
      (if (> (`KismetMathLibrary.VSize` (`self.GetVelocity`)) 20.0)
        (if (`self.IsTurning`)
          (bind _returnvalue_2 (`KismetMathLibrary.FindLookAtRotation` (`self.K2_GetActorLocation`) (`self.K2_GetActorLocation` _lock_target)))
          (bind (_returnvalue_roll _returnvalue_pitch _returnvalue_yaw) (`KismetMathLibrary.BreakRotator` (`KismetMathLibrary.RInterpTo` _returnvalue _returnvalue_2 (`GameplayStatics.GetWorldDeltaSeconds`) 3.0)))
          (`self.K2_SetActorRotation` (`KismetMathLibrary.MakeRotator` 0.0 0.0 _returnvalue_yaw)))
        (else
          (bind (_returnvalue_roll_2 _returnvalue_pitch_2 _returnvalue_yaw_2) (`KismetMathLibrary.BreakRotator` (`KismetMathLibrary.NormalizedDeltaRotator` _returnvalue _returnvalue_2)))
          (bind _returnvalue_3 (`KismetMathLibrary.Abs` _returnvalue_yaw_2))
          (if (and (> _returnvalue_3 85.0) (< _returnvalue_3 135.0))
            (`/Engine/EditorBlueprintResources/StandardMacros.DoOnce` false :!label _label
              (:`Completed`
                (`|PlayMontage` (`self.Mesh`) (select `bool` (> _returnvalue_yaw_2 0.0) :`false` "/Game/_MazeLong/EnemyTest/ImposterBeast/MoveSet/Rotate/ImposterBeast_Anim_Armature_CA_M_ImposterBeast_Turn_R_Montage.ImposterBeast_Anim_Armature_CA_M_ImposterBeast_Turn_R_Montage" :`true` "/Game/_MazeLong/EnemyTest/ImposterBeast/MoveSet/Rotate/ImposterBeast_Anim_Armature_CA_M_ImposterBeast_Turn_L_Montage.ImposterBeast_Anim_Armature_CA_M_ImposterBeast_Turn_L_Montage" :!type "AnimMontage Object Reference")
                  (:`OnCompleted`
                    (goto _label :!via `Reset`))
                  (:`OnInterrupted`
                    (goto _label :!via `Reset`)))))
            (else
              (bind _returnvalue_4 (`KismetMathLibrary.Abs` _returnvalue_yaw_2))
              (if (> _returnvalue_4 135.0)
                (`/Engine/EditorBlueprintResources/StandardMacros.DoOnce` false :!label _label_2
                  (:`Completed`
                    (`|PlayMontage` (`self.Mesh`) (select `bool` (> _returnvalue_4 0.0) :`false` "/Game/_MazeLong/EnemyTest/ImposterBeast/MoveSet/Rotate/ImposterBeast_Anim_Armature_CA_M_ImposterBeast_Turn_R_180_Montage.ImposterBeast_Anim_Armature_CA_M_ImposterBeast_Turn_R_180_Montage" :`true` "/Game/_MazeLong/EnemyTest/ImposterBeast/MoveSet/Rotate/ImposterBeast_Anim_Armature_CA_M_ImposterBeast_Turn_L_180_Montage.ImposterBeast_Anim_Armature_CA_M_ImposterBeast_Turn_L_180_Montage" :!type "AnimMontage Object Reference")
                      (:`OnCompleted`
                        (goto _label_2 :!via `Reset`))
                      (:`OnInterrupted`
                        (goto _label_2 :!via `Reset`)))))))))))
    (:`else`)))

(event `Attack2`
  (`|PlayMontage` (`self.Mesh`) "/Game/_MazeLong/EnemyTest/ImposterBeast/MoveSet/Atk/ImposterBeast_DoubleSwing_Montage.ImposterBeast_DoubleSwing_Montage"
    (:`OnCompleted`
      _)
    (:`OnInterrupted`
      _))
  (`self.On Anim End`))

(event `BackStep`
  (`|PlayMontage` (`self.Mesh`) "/Game/_MazeLong/EnemyTest/ImposterBeast/MoveSet/Atk/ImposterBeast_BackStep_Montage.ImposterBeast_BackStep_Montage"
    (:`OnCompleted`
      _)
    (:`OnInterrupted`
      _))
  (`self.On Anim End`))

(event `Attack`
  (`|PlayMontage` (`self.Mesh`) "/Game/_MazeLong/EnemyTest/ImposterBeast/MoveSet/Atk/ImposterBeast_CounterAtk_Montage.ImposterBeast_CounterAtk_Montage"
    (:`OnCompleted`
      _)
    (:`OnInterrupted`
      _))
  (`self.On Anim End`))

(event `AttackFreezy`
  (`/Engine/EditorBlueprintResources/StandardMacros.DoOnce` false :!label _label_3
    (:`Completed`
      (`|PlayMontage` (`self.Mesh`) "/Game/_MazeLong/EnemyTest/ImposterBeast/MoveSet/Atk/ImposterBeast_Frenzy_ChaosStomp_Jump_Start_Montage.ImposterBeast_Frenzy_ChaosStomp_Jump_Start_Montage"
        (:`OnCompleted`
          _)
        (:`OnInterrupted`
          _))
      (`|ExecutionSequence`
        (:`then_0`
          (goto _label_3 :!via `Reset`))
        (:`then_1`
          (`self.On Anim End`))))))

(event `JumpToPlayer`
  (`/Engine/EditorBlueprintResources/StandardMacros.DoOnce` false :!label _label_4
    (:`Completed`
      (`|PlayMontage` (`self.Mesh`) "/Game/_MazeLong/EnemyTest/ImposterBeast/MoveSet/Atk/ImposterBeast_ChaosStomp_Jump_Montage.ImposterBeast_ChaosStomp_Jump_Montage"
        (:`OnCompleted`
          _)
        (:`OnInterrupted`
          _))
      (`|ExecutionSequence`
        (:`then_0`
          (goto _label_4 :!via `Reset`))
        (:`then_1`
          (`self.On Anim End`))))))

(event `Roar`
  (`|PlayMontage` (`self.Mesh`) "/Game/_MazeLong/EnemyTest/ImposterBeast/MoveSet/Atk/ImposterBeast_StaminaReCharge_Montage.ImposterBeast_StaminaReCharge_Montage"
    (:`OnCompleted`
      _)
    (:`OnInterrupted`
      _))
  (`self.On Anim End`))

(event `self.ReceiveAnyDamage`
  (params (Damage :type "Float (single-precision)") (DamageType :type "DamageType Object Reference") (InstigatedBy :type "Controller Object Reference") (DamageCauser :type "Actor Object Reference"))
  (if (not (`self.Death?`))
    (bind _output_get (set `self.CurrentHealth` (`KismetMathLibrary.FClamp` (- (`self.CurrentHealth`) Damage) 0.0 (`self.MaxHealth`))))
    (bind _ui_info (`self.UI_Info`)
      (:`then`
        (`/Game/_MazeLong/_System/MazeLong_Info_Bar.UpdateBossHealth_UI` _ui_info _output_get (`self.MaxHealth`))
        (if (== (`self.CurrentHealth`) 0.0)
          (`self.Death`)))
      (:`else`))))

(event `Death`
  (bind _charactermovement (`self.CharacterMovement`))
  (set `self.Death?` true)
  (if (not (`self.ChetRoi`))
    (`SkeletalMeshComponent.PlayAnimation` (`self.Mesh`) "/Game/_MazeLong/EnemyTest/ImposterBeast/MoveSet/ImposterBeast_Die_F.ImposterBeast_Die_F" false)
    (`MovementComponent.StopMovementImmediately` _charactermovement)
    (`CharacterMovementComponent.DisableMovement` _charactermovement)
    (`PrimitiveComponent.SetCollisionResponseToAllChannels` (`self.CapsuleComponent`) "ECR_Ignore")))

(fn `Dead?`
  (returns (`Dead?` :type Boolean))
  (return (`self.Death?`)))

(fn `GetRef`
  (returns (Ref :type "Actor Object Reference"))
  (return null))

(fn `SetMovementSpeed`
  (params (MovementSpeed :type Byte :default 0))
  (returns (Speed :type "Float (double-precision)"))
  (return 0.0))

(fn `TakingDamaged`
  (returns (`Atked?` :type Boolean))
  (return false))

(fn `UpdateHealth`
  (if (not (`self.Death?`))
    (bind _output_get (set `self.CurrentHealth` (`KismetMathLibrary.FClamp` (+ (`self.HealthRegen`) (`self.CurrentHealth`)) 0.0 (`self.MaxHealth`))))
    (bind _ui_info (`self.UI_Info`)
      (:`then`
        _)
      (:`else`))
    (else
      (set `self.CurrentHealth` (`self.CurrentHealth`))))
  (`/Game/_MazeLong/_System/MazeLong_Info_Bar.UpdateBossHealth_UI` _ui_info _output_get (`self.MaxHealth`)))

(fn `UserConstructionScript`)