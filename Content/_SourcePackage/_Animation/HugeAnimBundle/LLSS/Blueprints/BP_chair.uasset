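; Placeable chair that characters with a BP_LLSS_Comp can sit on, using a trigger volume to feed that component.
; On overlap, if the component is not in transition and is in the required pose type, it receives the sit type, chair reference and target transform turned 180° in yaw, and its bed and wall references are cleared.
; Leaving clears InVolume.
; The construction script sets the mesh and shows a pose-number label when ForcedPose is on.
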(event `self.Trigger.OnComponentBeginOverlap`
  (params (OverlappedComponent :type "PrimitiveComponent Object Reference") (OtherActor :type "Actor Object Reference") (OtherComp :type "PrimitiveComponent Object Reference") (OtherBodyIndex :type Integer) (bFromSweep :type Boolean) (SweepResult :type "HitResult Structure (by ref)"))
  (bind _returnvalue (`SceneComponent.K2_GetComponentToWorld` (`self.Traget`)))
  (bind _ascharacter (cast `Character` OtherActor))
  (bind _returnvalue_2 (`self.GetComponentByClass` _ascharacter "/Game/_SourcePackage/_Animation/HugeAnimBundle/LLSS/Blueprints/BP_LLSS_Comp.BP_LLSS_Comp_C"))
  (`/Engine/EditorBlueprintResources/StandardMacros.IsValid` _returnvalue_2
    (:`Is Valid`
      (if (and (not (`/Game/_SourcePackage/_Animation/HugeAnimBundle/LLSS/Blueprints/BP_LLSS_Comp.InTransition` _returnvalue_2)) (`|EnumEquality` (`/Game/_SourcePackage/_Animation/HugeAnimBundle/LLSS/Blueprints/BP_LLSS_Comp.PoseType` _returnvalue_2) "NewEnumerator0"))
        (set `/Game/_SourcePackage/_Animation/HugeAnimBundle/LLSS/Blueprints/BP_LLSS_Comp.SitType` (`self.SitType`) _returnvalue_2)
        (set `/Game/_SourcePackage/_Animation/HugeAnimBundle/LLSS/Blueprints/BP_LLSS_Comp.ObjectTransforms` (`KismetMathLibrary.MakeTransform` (.location _returnvalue) (`KismetMathLibrary.MakeRotator` (.roll (.rotation _returnvalue)) (.pitch (.rotation _returnvalue)) (+ (.yaw (.rotation _returnvalue)) 180.0))) _returnvalue_2)
        (set `/Game/_SourcePackage/_Animation/HugeAnimBundle/LLSS/Blueprints/BP_LLSS_Comp.InVolume` true _returnvalue_2)
        (set `/Game/_SourcePackage/_Animation/HugeAnimBundle/LLSS/Blueprints/BP_LLSS_Comp.OverlappedChair` self _returnvalue_2)
        (set `/Game/_SourcePackage/_Animation/HugeAnimBundle/LLSS/Blueprints/BP_LLSS_Comp.OverlappedBed` null _returnvalue_2)
        (set `/Game/_SourcePackage/_Animation/HugeAnimBundle/LLSS/Blueprints/BP_LLSS_Comp.OverlappedWall` null _returnvalue_2)
        (set `/Game/_SourcePackage/_Animation/HugeAnimBundle/LLSS/Blueprints/BP_LLSS_Comp.VolumeType` "NewEnumerator4" _returnvalue_2)))))

(event `self.Trigger.OnComponentEndOverlap`
  (params (OverlappedComponent :type "PrimitiveComponent Object Reference") (OtherActor :type "Actor Object Reference") (OtherComp :type "PrimitiveComponent Object Reference") (OtherBodyIndex :type Integer))
  (bind _ascharacter (cast `Character` OtherActor))
  (set `/Game/_SourcePackage/_Animation/HugeAnimBundle/LLSS/Blueprints/BP_LLSS_Comp.InVolume` false (`self.GetComponentByClass` _ascharacter "/Game/_SourcePackage/_Animation/HugeAnimBundle/LLSS/Blueprints/BP_LLSS_Comp.BP_LLSS_Comp_C")))

(fn `UserConstructionScript`
  (bind _textrender (`self.TextRender`))
  (`SceneComponent.SetVisibility` _textrender (`self.ForcedPose`) false)
  (`TextRenderComponent.K2_SetText` _textrender (`KismetTextLibrary.Conv_StringToText` (`KismetStringLibrary.Concat_StrStr` "" " No " (`KismetStringLibrary.Conv_IntToString` (`self.PoseNo`)))))
  (`StaticMeshComponent.SetStaticMesh` (`self.Mesh`) (`self.MainMesh`)))