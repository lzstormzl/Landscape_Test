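; Skybox actor Blueprint for a static sky, whose BeginPlay, rotation events and Construction Script all do nothing.
; Disconnected Construction Script nodes would create a dynamic sky material and use DayNight to blend sky, sun, skylight and fog settings, with optional texture swaps.
; Unwired event-graph nodes hold a timer-based yaw rotation of the sky mesh, so none of this logic runs.
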(event `self.ReceiveBeginPlay`
  ;[0 0 1] Begin
)

(event `RotateSkybox`
  ;[1 1 1] Rotate Sky Animation
)

(event `Rotate`
  ;[1 1 1] Rotate Sky Animation
)

(fn `UserConstructionScript`)